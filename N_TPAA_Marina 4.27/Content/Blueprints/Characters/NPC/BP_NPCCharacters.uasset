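; BP_NPCCharacters is an NPC character Blueprint that hooks itself up to an on-screen health bar.
; On BeginPlay it casts the WidgetHP component's user widget to W_HealthBar and passes itself in as the character whose HP the bar tracks.
; Overlap and Tick events are disabled stubs, and the construction script only calls the parent.
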(event `self.ReceiveBeginPlay`
  (`parent.ReceiveBeginPlay`)
  (bind _asw_health_bar (cast `/Game/Blueprints/HUD/Widgets/W_HealthBar` (`WidgetComponent.GetUserWidgetObject` (`self.WidgetHP`))))
  (`/Game/Blueprints/HUD/Widgets/W_HealthBar.Update Current Character for HP` _asw_health_bar self))

(fn `UserConstructionScript`
  (`parent.UserConstructionScript`))