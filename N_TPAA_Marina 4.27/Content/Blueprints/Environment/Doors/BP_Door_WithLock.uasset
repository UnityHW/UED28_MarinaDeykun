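; BP_Door_WithLock is a child door Blueprint that adds a lock, shown by a red or green indicator light.
; Interact toggles an unlocked door; when locked, it checks the overlapping actor's backpack component for the required quest-item keys.
; Matching keys are removed as found, even from an incomplete set, and the door unlocks without opening only if all are found.
; Lock only takes effect on doors without required keys.
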(event `self.OpenDoor`
  (if (not (`self.IsLocked`))
    (`parent.OpenDoor`)))

(event `self.CloseDoor`
  (`parent.CloseDoor`))

(fn `Interact`
  (returns (Succes :type Boolean))
  (locals (L_Backpack :type "/Game/Blueprints/Components/BP_BackpackComponent Object Reference") (L_ItemInrement :type Integer) (L_ItemName :type Name))
  (if (`self.IsReadyToInteract`)
    (if (not (`self.IsLocked`))
      (if (`self.IsOpen`)
        (`self.CloseDoor`)
        (return true)
        (else
          (`self.OpenDoor`)
          (return true)))
      (elif (`KismetArrayLibrary.Array_IsValidIndex` (`self.NeededKeysName`))
        (bind _overlappedactor (`self.OverlappedActor`)
          (:`then`
            (bind _returnvalue (`self.GetComponentByClass` _overlappedactor "/Game/Blueprints/Components/BP_BackpackComponent.BP_BackpackComponent_C"))
            (`/Engine/EditorBlueprintResources/StandardMacros.IsValid` _returnvalue
              (:`Is Valid`
                (set `local.L_Backpack` _returnvalue)
                (for _array_element (`self.NeededKeysName`)
                  (set `local.L_ItemName` _array_element)
                  (if (`BlueprintSetLibrary.Set_Contains` (`/Game/Blueprints/Components/BP_BackpackComponent.QuestItems` (`local.L_Backpack`)) (`local.L_ItemName`))
                    (`/Engine/EditorBlueprintResources/StandardMacros.IncrementInt` (`local.L_ItemInrement`)
                      (:`  `
                        (`/Game/Blueprints/Components/BP_BackpackComponent.RemoveQuestItem` (`local.L_Backpack`) (`local.L_ItemName`))))))
                (if (== (`local.L_ItemInrement`) (`KismetArrayLibrary.Array_Length` (`self.NeededKeysName`)))
                  (`self.Unlock`)
                  (else
                    (return true))))
              (:`Is Not Valid`
                (return true))))
          (:`else`
            (return true)))
        (else
          (return true))))
    (else
      (return false))))

(fn `Lock`
  (if (not (`KismetArrayLibrary.Array_IsValidIndex` (`self.NeededKeysName`)))
    (set `self.IsLocked` true)
    (`self.UpdateDoorLockIndicaton`)))

(fn `SwitchLock`
  (set `self.IsLocked` (not (`self.IsLocked`)))
  (`self.UpdateDoorLockIndicaton`))

(fn `Unlock`
  (set `self.IsLocked` false)
  (`self.UpdateDoorLockIndicaton`))

(fn `UpdateDoorLockIndicaton`
  (`LightComponent.SetLightColor` (`self.LockIndicatorLight`) (`KismetMathLibrary.SelectColor` (struct :`R` 1.0 :`G` 0.003677 :`B` 0.003677 :`A` 1.0) (struct :`R` 0.040915 :`G` 0.863157 :`B` 0.078187 :`A` 1.0) (`self.IsLocked`)) true))

(fn `UserConstructionScript`
  (`parent.UserConstructionScript`)
  (`self.UpdateDoorLockIndicaton`))