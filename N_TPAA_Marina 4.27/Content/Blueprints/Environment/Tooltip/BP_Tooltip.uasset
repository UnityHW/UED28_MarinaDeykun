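; BP_Tooltip is a placeable actor that shows an in-world text tooltip while a Character stands inside its trigger box.
; Begin and end overlap events cast the other actor to Character, then unhide or hide the TooltipText component.
; The construction script sizes BoxCollision from the BoxExtent variable, raises it by its half-height to sit on the actor origin, and positions the text from TooltipTextLocation.
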(event `self.ReceiveActorBeginOverlap`
  (params (OtherActor :type "Actor Object Reference"))
  (cast `Character` OtherActor)
  (`SceneComponent.SetHiddenInGame` (`self.TooltipText`) false false))

(event `self.ReceiveActorEndOverlap`
  (params (OtherActor :type "Actor Object Reference"))
  (cast `Character` OtherActor)
  (`SceneComponent.SetHiddenInGame` (`self.TooltipText`) true false))

(fn `UserConstructionScript`
  (`BoxComponent.SetBoxExtent` (`self.BoxCollision`) (`self.BoxExtent`) true)
  (`SceneComponent.K2_SetRelativeLocation` (`self.BoxCollision`) (`KismetMathLibrary.MakeVector` 0.0 0.0 (.z (`self.BoxExtent`))) false false)
  (`SceneComponent.K2_SetRelativeLocation` (`self.TooltipText`) (`self.TooltipTextLocation`) false false))