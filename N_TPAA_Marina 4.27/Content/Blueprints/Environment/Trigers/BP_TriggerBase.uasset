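; BP_TriggerBase is a trigger volume actor, named as a base for environment triggers.
; The construction script sizes its box collision from BoxExtent and raises it by the Z extent so its bottom sits at the actor origin.
; Beginning an overlap stores the other actor in OverlappedActor, with no clearing on exit.
; Interact simply returns true, with no other behavior.
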(event `self.ReceiveActorBeginOverlap`
  (params (OtherActor :type "Actor Object Reference"))
  (set `self.OverlappedActor` OtherActor))

(fn `Interact`
  (returns (Succes :type Boolean))
  (return true))

(fn `UserConstructionScript`
  (`BoxComponent.SetBoxExtent` (`self.BoxCollision`) (`self.BoxExtent`) true)
  (`SceneComponent.K2_SetRelativeLocation` (`self.BoxCollision`) (`KismetMathLibrary.MakeVector` 0.0 0.0 (.z (`self.BoxExtent`))) false false))