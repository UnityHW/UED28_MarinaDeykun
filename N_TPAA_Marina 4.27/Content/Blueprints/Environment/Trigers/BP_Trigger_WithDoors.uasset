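; BP_Trigger_WithDoors is an environment trigger that toggles the locks on a set of doors when the player character type overlaps it.
; On overlap it runs the parent handler, then checks that OverlappedActor is valid and casts it to ThirdPersonCharacter.
; SwitchDoorsLocks then calls SwitchLock on every entry in DoorsToLockSwitch, flipping each lock rather than setting a fixed state.
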(event `self.ReceiveActorBeginOverlap`
  (params (OtherActor :type "Actor Object Reference"))
  (`parent.ReceiveActorBeginOverlap` OtherActor)
  (bind _overlappedactor (`self.OverlappedActor`)
    (:`then`
      (cast `/Game/Blueprints/Characters/ThirdPersonCharacter` _overlappedactor)
      (`self.SwitchDoorsLocks`))
    (:`else`)))

(fn `SwitchDoorsLocks`
  (for _array_element (`self.DoorsToLockSwitch`)
    (`/Game/Blueprints/Environment/Doors/BP_Door_WithLock.SwitchLock` _array_element)))

(fn `UserConstructionScript`
  (`parent.UserConstructionScript`))