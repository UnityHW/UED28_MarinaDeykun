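; BP_TestA is a test actor that displays text on a TextRender component.
; The construction script formats MyName into a "My name is" label.
; On BeginPlay it replaces the label with the TrafficLight enum as text, then steps through two further values with two-second delays, without looping.
; The rest is disconnected experiments with array and map variables, debug visibility and print strings, none of which run.
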(event `self.ReceiveBeginPlay`
  (`TextRenderComponent.K2_SetText` (`self.TextRender`) (`|FormatText` (`KismetTextLibrary.Conv_StringToText` (`|GetEnumeratorNameAsString` (`self.Traffic light`)))))
  (`KismetSystemLibrary.Delay` 2.0)
  (set `self.Traffic light` "NewEnumerator1")
  (`TextRenderComponent.K2_SetText` (`self.TextRender`) (`|FormatText` (`KismetTextLibrary.Conv_StringToText` (`|GetEnumeratorNameAsString` (`self.Traffic light`)))))
  (`KismetSystemLibrary.Delay` 2.0)
  (set `self.Traffic light` "NewEnumerator2")
  (`TextRenderComponent.K2_SetText` (`self.TextRender`) (`|FormatText` (`KismetTextLibrary.Conv_StringToText` (`|GetEnumeratorNameAsString` (`self.Traffic light`))))))

(event `self.ReceiveTick`
  (params (DeltaSeconds :type "Float (single-precision)")))

(fn `UserConstructionScript`
  (`TextRenderComponent.K2_SetText` (`self.TextRender`) (`|FormatText` "My name is {Name}" (`self.My name`))))